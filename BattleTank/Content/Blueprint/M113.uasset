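; M113 tracked vehicle Blueprint that supplies components and setup data to a parent tank class with C++ pointers.
; Construction builds five suspension entries per side from handle transforms and per-side setup arrays.
; BeginPlay binds body, sweep, tread and spline references, creates dynamic tread materials and assigns the Detroit 6V53T torque curve.
; It also fills wheel, sprocket and idler arrays and registers the turret and barrel.
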(event EventBeginPlay
  (Utilities|FlowControl|Sequence
    (:then_0
      ;[1 1 1] Initialize C++ pointers
      (Variables|Default|SetBody (Variables|Default|GetBP_Body))
      (Variables|Default|SetCOM (Variables|Default|GetBP_COM))
      (Variables|Default|SetWheelSweep (Variables|Default|GetBP_WheelSweep))
      (Variables|Default|SetTreadR (Variables|Default|GetBP_TreadsR))
      (Variables|Default|SetTreadL (Variables|Default|GetBP_TreadsL))
      (Variables|Default|SetTrackSplineR (Variables|Default|GetTrackSplineR_0))
      (Variables|Default|SetTrackSplineL (Variables|Default|GetTrackSplineL_0))
      (bind _returnvalue (Rendering|Material|CreateDynamicMaterialInstance "/Game/Materials/M_Tread_Inst.M_Tread_Inst" :!class /Script/Engine.KismetMaterialLibrary))
      (Variables|Default|SetTreadMaterialRight _returnvalue)
      (bind _returnvalue_2 (Rendering|Material|CreateDynamicMaterialInstance "/Game/Materials/M_Tread_Inst.M_Tread_Inst" :!class /Script/Engine.KismetMaterialLibrary))
      (Variables|Default|SetTreadMaterialLeft _returnvalue_2)
      (Rendering|Material|SetMaterial (Variables|Default|GetBP_TreadR) 0 (Variables|Default|GetTreadMaterialRight))
      (Rendering|Material|SetMaterial (Variables|Default|GetBP_TreadL) 0 (Variables|Default|GetTreadMaterialLeft))
      (Variables|Default|SetEngineTorqueCurve "/Game/Blueprint/Curves/Detroit_6V53T.Detroit_6V53T"))
    (:then_1
      (CallFunction|InitializeWheels)
      (CallFunction|InitializeSprockets)
      (CallFunction|InitializeIdlers)
      (Class|TrackedVehicle|SetBarrelReference (Variables|Default|GetTankBarrel))
      (Class|TrackedVehicle|SetTurretReference (Variables|Default|GetTankTurret)))))

(event Collision|EventActorBeginOverlap
  (params (OtherActor :type Actor%20Object%20Reference)))

(event EventTick
  (params (DeltaSeconds :type Float%20%28single-precision%29)))

(fn ConstructionScript
  (|CallParentFunction)
  (CallFunction|ConstructSups))

(fn RegisterSuspensionHandles
  (bind _susphandleright (Variables|Default|GetSuspHandleRight))
  (bind _susphandleleft (Variables|Default|GetSuspHandleLeft))
  (Utilities|Array|Clear _susphandleright)
  (Utilities|Array|Add _susphandleright (Variables|Default|GetSuspR01))
  (Utilities|Array|Add _susphandleright (Variables|Default|GetSuspR02))
  (Utilities|Array|Add _susphandleright (Variables|Default|GetSuspR03))
  (Utilities|Array|Add _susphandleright (Variables|Default|GetSuspR04))
  (Utilities|Array|Add _susphandleright (Variables|Default|GetSuspR05))
  (Utilities|Array|Clear _susphandleleft)
  (Utilities|Array|Add _susphandleleft (Variables|Default|GetSuspL01))
  (Utilities|Array|Add _susphandleleft (Variables|Default|GetSuspL02))
  (Utilities|Array|Add _susphandleleft (Variables|Default|GetSuspL03))
  (Utilities|Array|Add _susphandleleft (Variables|Default|GetSuspL04))
  (Utilities|Array|Add _susphandleleft (Variables|Default|GetSuspL05))
  (return false))

(fn BuildTrackSpline
  (params (SplineR :type Spline%20Component%20Object%20Reference) (SplineL :type Spline%20Component%20Object%20Reference) (TreadsR :type Instanced%20Static%20Mesh%20Component%20Object%20Reference) (TreadsL :type Instanced%20Static%20Mesh%20Component%20Object%20Reference))
  (bind _output_get (Variables|Default|SetTreadR (Variables|Default|GetBP_TreadsR)))
  (bind _output_get_2 (Variables|Default|SetTreadL (Variables|Default|GetBP_TreadsL)))
  (bind _dummy (|CallParentFunction (Variables|Default|GetTrackSplineR_0) (Variables|Default|GetTrackSplineL_0) _output_get _output_get_2))
  (return _dummy))

(fn InitializeSprockets
  (bind _sprocketsright (Variables|Default|GetSprocketsRight))
  (bind _sprocketsleft (Variables|Default|GetSprocketsLeft))
  (Utilities|Array|Clear _sprocketsright)
  (Utilities|Array|Add _sprocketsright (Variables|Default|GetSprockerR))
  (Utilities|Array|Clear _sprocketsleft)
  (Utilities|Array|Add _sprocketsleft (Variables|Default|GetSprockerL)))

(fn InitializeWheels
  (Utilities|Array|Clear (Variables|Default|GetRightWheels))
  (Utilities|Array|Clear (Variables|Default|GetLeftWheels))
  (for (_ _array_index) (Variables|Default|GetSuspensionsInternalRight)
    (Utilities|Array|Add (Variables|Default|GetRightWheels) (Utilities|Select :Index _array_index :Option%200 (Variables|Default|GetR01) :Option%201 (Variables|Default|GetR02) :Option%202 (Variables|Default|GetR03) :Option%203 (Variables|Default|GetR04) :Option%204 (Variables|Default|GetR05))))
  (for (_ _array_index_2) (Variables|Default|GetSuspensionsInternalLeft)
    (Utilities|Array|Add (Variables|Default|GetLeftWheels) (Utilities|Select :Index _array_index_2 :Option%200 (Variables|Default|GetL01) :Option%201 (Variables|Default|GetL02) :Option%202 (Variables|Default|GetL03) :Option%203 (Variables|Default|GetL04) :Option%204 (Variables|Default|GetL05)))))

(fn InitializeIdlers
  (bind _idlersright (Variables|Default|GetIdlersRight))
  (bind _idlersleft (Variables|Default|GetIdlersLeft))
  (Utilities|Array|Clear _idlersright)
  (Utilities|Array|Clear _idlersleft)
  (Utilities|Array|Add _idlersright (Variables|Default|GetIdlerR))
  (Utilities|Array|Add _idlersleft (Variables|Default|GetIdlerL)))

(fn ConstructSups
  (for (_array_element _array_index) (Variables|Default|GetSuspHandleRight)
    (Utilities|Array|Add (Variables|Default|GetSuspensionsInternalRight) (Utilities|Struct|MakeSuspensionInternalProcessing (.location (Transformation|GetRelativeTransform _array_element)) (.rotation (Transformation|GetRelativeTransform _array_element)) (.maximumlength (Utilities|Array|Get(acopy) (Variables|Default|GetFSuspensionSetupR) _array_index)) (.collisionradius (Utilities|Array|Get(acopy) (Variables|Default|GetFSuspensionSetupR) _array_index)) (.stiffnessforce (Utilities|Array|Get(acopy) (Variables|Default|GetFSuspensionSetupR) _array_index)) (.dampingforce (Utilities|Array|Get(acopy) (Variables|Default|GetFSuspensionSetupR) _array_index)) 0.0 "0, 0, 0" "0, 0, 0" "0, 0, 0" false "SurfaceType_Default")))
  (for (_array_element_2 _array_index_2) (Variables|Default|GetSuspHandleLeft)
    (Utilities|Array|Add (Variables|Default|GetSuspensionsInternalLeft) (Utilities|Struct|MakeSuspensionInternalProcessing (.location (Transformation|GetRelativeTransform _array_element_2)) (.rotation (Transformation|GetRelativeTransform _array_element_2)) (.maximumlength (Utilities|Array|Get(acopy) (Variables|Default|GetFSuspensionSetupL) _array_index_2)) (.collisionradius (Utilities|Array|Get(acopy) (Variables|Default|GetFSuspensionSetupL) _array_index_2)) (.stiffnessforce (Utilities|Array|Get(acopy) (Variables|Default|GetFSuspensionSetupL) _array_index_2)) (.dampingforce (Utilities|Array|Get(acopy) (Variables|Default|GetFSuspensionSetupL) _array_index_2)) 0.0 "0, 0, 0" "0, 0, 0" "0, 0, 0" false "SurfaceType_Default"))))