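; Tracked vehicle Blueprint that turns player input into drive, steering and brake coefficients and orbits an aim camera via gimbal and spring arm.
; Steering sets opposing left/right wheel coefficients; forward input feeds either auto-handling throttle or manual throttle and braking.
; Construction precomputes sprocket and track inertia, shows center of mass, selects the starting gear, and spaces instanced treads evenly along both track splines.
; Suspension registration and simple-track material functions are empty stubs here.
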(event EventBeginPlay)

(event Collision|EventActorBeginOverlap
  (params (OtherActor :type Actor%20Object%20Reference)))

(event EventTick
  (params (DeltaSeconds :type Float%20%28single-precision%29)))

(event Input|AxisEvents|InputAxisFWD
  (params (AxisValue :type Float%20%28single-precision%29))
  (bind _returnvalue (< AxisValue 0.0))
  (bind _returnvalue_2 (select _returnvalue -1.0 0.0))
  (bind _returnvalue_3 (* AxisValue _returnvalue_2))
  (if (Variables|Default|GetAutoGearBox)
    (Class|TrackedVehicle|GetThrottleInputforAutoHandling (stale Input|AxisEvents|InputAxisRotate AxisValue) AxisValue)
    (if (or (!= (stale Input|AxisEvents|InputAxisRotate AxisValue) 0.0) (!= AxisValue 0.0))
      (Variables|Default|SetSleepMod false)
      (Variables|Default|SetSleepDelayTimer 0.0))
    (else
      (Variables|Default|SetWheelForwardCoefficient (Math|Float|Clamp(Float) AxisValue))
      (Variables|Default|SetBrakeRatioRight _returnvalue_3)
      (Variables|Default|SetBrakeRatioLeft _returnvalue_3))))

(event Input|AxisEvents|InputAxisAimAzimuthX
  (params (AxisValue :type Float%20%28single-precision%29))
  (Transformation|AddLocalRotation (Variables|Default|GetAzimuthGimbal) (Math|Rotator|MakeRotator 0.0 0.0 (* AxisValue (Utilities|Time|GetWorldDeltaSeconds) 1e+02)) false false))

(event Input|AxisEvents|InputAxisAimAzimuthY
  (params (AxisValue :type Float%20%28single-precision%29))
  (Transformation|AddLocalRotation (Variables|Default|GetSpringArm) (Math|Rotator|MakeRotator 0.0 (* AxisValue (Utilities|Time|GetWorldDeltaSeconds) 1e+02) 0.0) false false))

(event Input|AxisEvents|InputAxisRotate
  (params (AxisValue :type Float%20%28single-precision%29))
  (bind _returnvalue (Math|Float|Absolute(Float) AxisValue))
  (Variables|Default|SetWheelRightCoefficient (* _returnvalue (select (< AxisValue 0.0) 1.0 -1.0)))
  (Variables|Default|SetWheelLeftCoefficient (* _returnvalue (select (< AxisValue 0.0) -1.0 1.0)))
  (if (or (!= AxisValue 0.0) (!= (stale Input|AxisEvents|InputAxisFWD AxisValue) 0.0))
    (Variables|Default|SetSleepMod false)
    (Variables|Default|SetSleepDelayTimer 0.0)))

(fn ConstructionScript
  (Utilities|FlowControl|Sequence
    (:then_0
      (CallFunction|PreCalculateMomentOfIntertia))
    (:then_1
      (CallFunction|RegisterSuspensionHandles))
    (:then_2
      (CallFunction|VisualizeCenterOfMass))
    (:then_3
      (CallFunction|CreateMaterialsforSimpleTracks))
    (:then_4
      (CallFunction|BuildTrackSpline))
    (:then_5
      (bind _array_element (Utilities|Array|ForEachLoopwithBreak (Variables|Default|GetGearRatio) :!label _label)
        (:LoopBody
          (if (== _array_element 0.0)
            (Variables|Default|SetNeutralGearIndex 0)
            (goto _label Break)))
        (:Completed
          (Variables|Default|SetCurrentGear (Math|Integer|SelectInt (+ (Variables|Default|GetNeutralGearIndex) 1) (Variables|Default|GetNeutralGearIndex) (Variables|Default|GetAutoGearBox))))))))

(fn InitializeCpp)

(fn BuildTrackSpline
  (params (SplineR :type Spline%20Component%20Object%20Reference) (SplineL :type Spline%20Component%20Object%20Reference) (TreadsR :type Instanced%20Static%20Mesh%20Component%20Object%20Reference) (TreadsL :type Instanced%20Static%20Mesh%20Component%20Object%20Reference))
  (LocalVariables|SetSplineRLoc SplineR)
  (LocalVariables|SetSplineLLoc SplineL)
  (LocalVariables|SetTreadsRLoc TreadsR)
  (LocalVariables|SetTreadsLLoc TreadsL)
  (Variables|Default|SetTreadsLastIndex (Math|Float|Truncate (- (Variables|Default|GetTreadsOnSide) 1.0)))
  (Spline|SetSplinePoints (LocalVariables|GetSplineRLoc) (Variables|Default|GetSplineCoordinatesR) "Local" true)
  (Spline|SetSplinePoints (LocalVariables|GetSplineLLoc) (Variables|Default|GetSplineCoordinatesL) "Local" true)
  (for (_array_element _array_index) (Variables|Default|GetSplineTangents)
    (Spline|SetTangentatSplinePoint (LocalVariables|GetSplineRLoc) _array_index _array_element "Local" true)
    (Spline|SetTangentatSplinePoint (LocalVariables|GetSplineLLoc) _array_index _array_element "Local" true))
  (for _index (range 0 (Variables|Default|GetTreadsLastIndex))
    (Components|InstancedStaticMesh|AddInstance (LocalVariables|GetTreadsRLoc) (Math|Transform|MakeTransform (Spline|GetLocationatDistanceAlongSpline (LocalVariables|GetSplineRLoc) (* _index (/ (Spline|GetSplineLength (LocalVariables|GetSplineRLoc)) (Variables|Default|GetTreadsOnSide))) "Local") (Math|Rotator|MakeRotator (Math|Float|SelectFloat 1.8e+02 (.roll (Spline|GetRotationatDistanceAlongSpline (LocalVariables|GetSplineRLoc) (* _index (/ (Spline|GetSplineLength (LocalVariables|GetSplineRLoc)) (Variables|Default|GetTreadsOnSide))) "Local")) (< (.y (Class|SplineComponent|GetRightVectoratDistanceAlongSpline (LocalVariables|GetSplineRLoc) (* _index (/ (Spline|GetSplineLength (LocalVariables|GetSplineRLoc)) (Variables|Default|GetTreadsOnSide))) "Local")) 0.0)) (.pitch (Spline|GetRotationatDistanceAlongSpline (LocalVariables|GetSplineRLoc) (* _index (/ (Spline|GetSplineLength (LocalVariables|GetSplineRLoc)) (Variables|Default|GetTreadsOnSide))) "Local")) (.yaw (Spline|GetRotationatDistanceAlongSpline (LocalVariables|GetSplineRLoc) (* _index (/ (Spline|GetSplineLength (LocalVariables|GetSplineRLoc)) (Variables|Default|GetTreadsOnSide))) "Local"))) (Math|Vector|MakeVector 1.0 1.0 1.0)))
    (Variables|Default|SetSplineLengthAtConstruction (Spline|GetSplineLength (LocalVariables|GetSplineRLoc))))
  (for _index_2 (range 0 (Variables|Default|GetTreadsLastIndex))
    (Components|InstancedStaticMesh|AddInstance (LocalVariables|GetTreadsLLoc) (Math|Transform|MakeTransform (Spline|GetLocationatDistanceAlongSpline (LocalVariables|GetSplineLLoc) (* _index_2 (/ (Spline|GetSplineLength (LocalVariables|GetSplineLLoc)) (Variables|Default|GetTreadsOnSide))) "Local") (Math|Rotator|MakeRotator (Math|Float|SelectFloat 1.8e+02 (.roll (Spline|GetRotationatDistanceAlongSpline (LocalVariables|GetSplineLLoc) (* _index_2 (/ (Spline|GetSplineLength (LocalVariables|GetSplineLLoc)) (Variables|Default|GetTreadsOnSide))) "Local")) (< (.y (Class|SplineComponent|GetRightVectoratDistanceAlongSpline (LocalVariables|GetSplineLLoc) (* _index_2 (/ (Spline|GetSplineLength (LocalVariables|GetSplineLLoc)) (Variables|Default|GetTreadsOnSide))) "Local")) 0.0)) (.pitch (Spline|GetRotationatDistanceAlongSpline (LocalVariables|GetSplineLLoc) (* _index_2 (/ (Spline|GetSplineLength (LocalVariables|GetSplineLLoc)) (Variables|Default|GetTreadsOnSide))) "Local")) (.yaw (Spline|GetRotationatDistanceAlongSpline (LocalVariables|GetSplineLLoc) (* _index_2 (/ (Spline|GetSplineLength (LocalVariables|GetSplineLLoc)) (Variables|Default|GetTreadsOnSide))) "Local"))) (Math|Vector|MakeVector 1.0 1.0 1.0))))
  (return false))

(fn PreCalculateMomentOfIntertia
  (bind _sprocketradiuscm (Variables|Default|GetSprocketRadiusCm))
  (bind _returnvalue (* _sprocketradiuscm _sprocketradiuscm))
  (Variables|Default|SetMomentIntertia (+ (* (* (Variables|Default|GetSprocketMassKg) 0.5) _returnvalue) (* _returnvalue (Variables|Default|GetTrackMassKg)))))

(fn VisualizeCenterOfMass
  (bind _returnvalue (Physics|GetCenterOfMass (Variables|Default|GetBP_Body) "None"))
  (Transformation|SetWorldLocation (Variables|Default|GetBP_COM) _returnvalue false false))

(fn CreateMaterialsforSimpleTracks)

(fn RegisterSuspensionHandles
  (return false))